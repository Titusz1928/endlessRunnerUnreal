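; Game mode for a runner game that builds an endless floor from BP_Floor tiles and restores the saved coin count.
; BeginPlay spawns the initial tiles, loading Coins from the save slot inside the same loop, so the load repeats per tile.
; AddFloor chains each tile to the previous one's attach point.
; Extendfloor adds a tile and destroys the oldest once the array exceeds the initial count plus a fixed buffer.
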(event `self.ReceiveBeginPlay`
  (for _ (range (`self.nrOfTiles`))
    (`self.addFloor`)
    (bind _returnvalue (`GameplayStatics.LoadGameFromSlot` "CoinVlaue"))
    (bind _asrunner_save_game (cast `/Game/Runner/Blueprints/Runner_saveGame` _returnvalue))
    (set `self.Coins` (`/Game/Runner/Blueprints/Runner_saveGame.CoinVlaue` _asrunner_save_game))))

(fn `addFloor`
  (bind _returnvalue (`|SpawnActorFromClass` "/Game/Runner/Blueprints/BP_Floor.BP_Floor_C" (`self.spawn attach point`) "Undefined" "MultiplyWithRoot" null null))
  (bind _returnvalue_2 (`/Game/Runner/Blueprints/BP_Floor.getAttachPoint` _returnvalue))
  (set `self.spawn attach point` _returnvalue_2)
  (`KismetArrayLibrary.Array_Add` (`self.floortiles`) _returnvalue)
  (bind _result (`/Engine/EditorBlueprintResources/StandardMacros.IncrementInt` (`self.Floor Count`))
    (:`  `
      (set `self.Floor Count` _result))))

(fn `extendfloor`
  (bind _floortiles (`self.floortiles`))
  (bind _output (`|GetArrayItem` _floortiles))
  (`self.addFloor`)
  (if (> (`KismetArrayLibrary.Array_Length` (`self.floortiles`)) (+ (`self.nrOfTiles`) 10))
    (`self.K2_DestroyActor` _output)
    (`KismetArrayLibrary.Array_RemoveItem` _floortiles _output)))

(fn `UserConstructionScript`)