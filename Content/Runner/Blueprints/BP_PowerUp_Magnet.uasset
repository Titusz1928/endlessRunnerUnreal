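; Magnet power-up pickup for the runner game that temporarily turns on the player character's magnet state.
; On player overlap it plays a sound, hides itself and, if no magnet is active, sets the flag and the game mode's MagnetTimer.
; A delayed loop ticks that timer down each second, while a separate delay clears the flag and destroys the actor.
; Overlapping a wall obstacle also destroys the pickup.
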(event `self.ReceiveActorBeginOverlap`
  (params (OtherActor :type "Actor Object Reference"))
  (`|ExecutionSequence`
    (:`then_0`
      (bind _asbp_runner_character (cast `/Game/Runner/Blueprints/CharacterBPs/BP_RunnerCharacter` OtherActor))
      (bind _asbp_runner_game_mode (cast `/Game/Runner/Blueprints/BP_RunnerGameMode` (`GameplayStatics.GetGameMode`)))
      (`GameplayStatics.PlaySound2D` "/Game/Runner/Meshes/350874__cabled_mess__coin_c_08.350874__cabled_mess__coin_c_08" 1.0 1.0 0.0 null null)
      (`self.SetActorHiddenInGame` true)
      (if (not (`/Game/Runner/Blueprints/CharacterBPs/BP_RunnerCharacter.isMagnetActive` _asbp_runner_character))
        (set `/Game/Runner/Blueprints/CharacterBPs/BP_RunnerCharacter.isMagnetActive` true _asbp_runner_character)
        (set `/Game/Runner/Blueprints/BP_RunnerGameMode.Magnet Timer` 6.0 _asbp_runner_game_mode)
        (`|ExecutionSequence`
          (:`then_0`
            (`/Game/Runner/Blueprints/Inputs/ForLoopDelay.ForLoopWithDelay` 0 5 1.0
              (:`Loop Body`
                (bind _result (`/Engine/EditorBlueprintResources/StandardMacros.DecrementFloat` (`/Game/Runner/Blueprints/BP_RunnerGameMode.Magnet Timer` _asbp_runner_game_mode))
                  (:`  `
                    (set `/Game/Runner/Blueprints/BP_RunnerGameMode.Magnet Timer` (`KismetMathLibrary.FMax` _result) _asbp_runner_game_mode))))))
          (:`then_1`
            (`KismetSystemLibrary.Delay` 5.2)
            (bind _asbp_runner_character_2 (cast `/Game/Runner/Blueprints/CharacterBPs/BP_RunnerCharacter` (`GameplayStatics.GetPlayerCharacter` 0)))
            (set `/Game/Runner/Blueprints/CharacterBPs/BP_RunnerCharacter.isMagnetActive` false _asbp_runner_character_2)
            (`self.K2_DestroyActor`)))))
    (:`then_1`
      (cast `/Game/Runner/Blueprints/Obstacles/BP_Obstacles_Wall` OtherActor)
      (`self.K2_DestroyActor`))))

(fn `UserConstructionScript`)